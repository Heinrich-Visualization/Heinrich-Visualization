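; BP_BG is a Blueprint, apparently a background actor, that handles cursor setup and a duck kill check.
; BeginPlay shows the mouse cursor and calls Possess on the player controller with no pawn specified.
; Each Tick compares Duck to the HitActor of a hand-built HitResult holding the player controller, switching Duck to the FB_DucksKillL flipbook on a match.
; No trace or click detection feeds that check.
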(event EventBeginPlay
  (bind _returnvalue (Game|GetPlayerController 0))
  (Variables|/Script/Engine.PlayerController|SetbShowMouseCursor _returnvalue true)
  (Pawn|Possess _returnvalue))

(event EventTick
  (params (DeltaSeconds :type Float%20%28single-precision%29))
  (if (== (Variables|Default|GetDuck) (.hitactor (Collision|MakeHitResult false false 0.0 0.0 "0, 0, 0" "0, 0, 0" "0,0,1" "0,0,1" 0 (Game|GetPlayerController 0))))
    (Sprite|SetFlipbook (Variables|Default|GetDuck) "/Game/Sprites/Flipbook/FB_DucksKillL.FB_DucksKillL")))

(fn ConstructionScript)